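; Enemy AI controller that runs a behavior tree and turns sight and hearing perception into blackboard data.
; Sight sets the target actor or records the last location where it was lost.
; Heard sounds are weakened by wall line traces and distance, then stored with location and an alert-strength type.
; It also picks a random waypoint subset and builds random patrol routes or seek routes from waypoints nearest the lost target.
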(event OnTargetPerceptionUpdated(AIPerception)
  (params (Actor :type Actor%20Object%20Reference) (Stimulus :type AI%20Stimulus%20Structure))
  ;[0.1953 0 1] AI Perception
  (bind _returnvalue (Class|AIPerceptionSystem|GetSenseClassforStimulus Stimulus))
  (if (== _returnvalue "/Script/AIModule.AISense_Sight")
    (CallFunction|HandleSightStimulus Actor Stimulus)
    (else
      (CallFunction|HandleHearStimulus Actor Stimulus))))

(event EventBeginPlay
  ;[1 0.07031 0] Begin
  (CallFunction|FetchAllWaypoints)
  (CallFunction|DetermineUsableWaypoins)
  (AI|RunBehaviorTree (Variables|Blackboard|GetBTAsset)))

(fn ConstructionScript)

(fn FetchAllWaypoints
  (bind _outactors (Actor|GetAllActorsOfClass (Variables|Routing|GetWaypointClass)))
  (Variables|Routing|SetAllWaypoints _outactors))

(fn DetermineUsableWaypoins
  (CallFunction|AddRandomItemsfromSource (Variables|Routing|GetUsableWaypoints) (Variables|Routing|GetAllWaypoints) (CallFunction|ComputeUsableWaypointCount)))

(fn ComputeUsableWaypointCount
  (return (CallFunction|ComputeRandomIntinVector2d (Variables|Routing|GetUsableWaypointCountRange))))

(fn AddRandomUsableWaypoint
  (bind _allwaypoints (Variables|Routing|GetAllWaypoints))
  (bind _outitem (Utilities|Array|Random _allwaypoints))
  (Utilities|Array|Add (Variables|Routing|GetUsableWaypoints) _outitem)
  (Utilities|Array|RemoveItem _allwaypoints _outitem))

(fn ComputeRouteLength
  (return (CallFunction|ComputeRandomIntinVector2d (Variables|Routing|GetRouteLengthRange))))

(fn GetNearestWaypoint
  (params (Location :type Vector) (Waypoints :type Array%20of%20Actor%20Object%20References))
  (LocalVariables|SetNearestWaypointDistance 7.766279436516721e+18)
  (for _array_element Waypoints
    (Math|Float|CompareFloat (Math|Vector|Distance(Vector) (Transformation|GetActorLocation _array_element) Location) (LocalVariables|GetNearestWaypointDistance)
      (:<
        (LocalVariables|SetNearestWaypoint _array_element))))
  (return (LocalVariables|GetNearestWaypoint)))

(fn HandleSightStimulus
  (params (StimulustActor :type Actor%20Object%20Reference) (Stimulus :type AI%20Stimulus%20Structure))
  (bind (_stimuluslocation _bsuccessfullysensed) (Utilities|Struct|BreakAIStimulus Stimulus))
  (if _bsuccessfullysensed
    (CallFunction|UpdateTargetActor StimulustActor)
    (else
      (CallFunction|UpdateLostTargetData _stimuluslocation))))

(fn HandleHearStimulus
  (params (StimulusActor :type Actor%20Object%20Reference) (Stimulus :type AI%20Stimulus%20Structure))
  (bind (_age _expirationage _strength _stimuluslocation) (Utilities|Struct|BreakAIStimulus Stimulus))
  (bind __ (CallFunction|ProcessSoundStrength _strength _stimuluslocation))
  (Utilities|IsHearableSoundStrength? _strength
    (:Is%20Hearable
      (Development|PrintString (Utilities|String|ToString(Float) __))
      (Utilities|IsHearableSoundStrength? __
        (:Is%20Hearable
          (CallFunction|UpdateHeardShotLocation _stimuluslocation)
          (CallFunction|UpdateHeardShotStrengthType (CallFunction|ComputeHeardShotStrengthType __)))))))

(fn ProcessSoundStrength
  (params (SoundStrength :type Float%20%28single-precision%29) (SoundLocation :type Vector))
  (return (CallFunction|ProcessSoundStrengthwithDistanceDecay (CallFunction|ProcessSoundStrengthwithObstacleDecay SoundStrength SoundLocation) SoundLocation)))

(fn ComputeHeardShotStrengthType
  (params (SoundStrength :type Float%20%28single-precision%29))
  (bind _returnvalue (CallFunction|CheckIsSoundIsEnoughtoAlert? SoundStrength))
  (bind _returnvalue_2 (Utilities|Enum|LiteralenumBPE_HeardSoundStrength "NewEnumerator1"))
  (bind _returnvalue_3 (Utilities|Enum|LiteralenumBPE_HeardSoundStrength "NewEnumerator0"))
  (bind _returnvalue_4 (select _returnvalue _returnvalue_3 _returnvalue_2))
  (Development|PrintString (Utilities|String|EnumtoString _returnvalue_4))
  (return _returnvalue_4))

(fn ProcessSoundStrengthwithObstacleDecay
  (params (SoundStrength :type Float%20%28single-precision%29) (SoundLocation :type Vector))
  (bind _outhits (Class|KismetSystemLibrary|LineTraceMultiforObjects SoundLocation (Transformation|GetActorLocation (Pawn|GetControlledPawn)) (Utilities|Array|MakeArray "ObjectTypeQuery1") false 0 "None" true "(R=1.000000,G=0.000000,B=0.000000,A=1.000000)" "(R=0.000000,G=1.000000,B=0.000000,A=1.000000)" 1.0))
  (Development|PrintString (Utilities|String|Append (Utilities|String|ToString(Integer) (Utilities|Array|Length _outhits)) " Obstacles between sound and receiver"))
  (return (|(Strength-((min((ObstacleCount*DecayRatioByObstacle),1))*Strength)) SoundStrength (Variables|Default|GetSoundStrengthDecayRatioByObstacle) (Utilities|Array|Length _outhits))))

(fn ProcessSoundStrengthwithDistanceDecay
  (params (SoundStrength :type Float%20%28single-precision%29) (SoundLocation :type Vector))
  (return (- SoundStrength (* (Math|Vector|Distance(Vector) SoundLocation (Transformation|GetActorLocation (Pawn|GetControlledPawn))) (Variables|Default|GetSoundStrengthDecayByDistance)))))

(fn UpdateTargetActor
  (params (TargetActor :type Actor%20Object%20Reference))
  (AI|Components|Blackboard|SetValueasObject (Variables|Default|GetBlackboard) (Variables|Blackboard|GetTargetActorBBKey) TargetActor)
  (return))

(fn UpdateLostTargetLocation
  (params (VectorValue :type Vector))
  (AI|Components|Blackboard|SetValueasVector (Variables|Default|GetBlackboard) (Variables|Blackboard|GetLostTargetLocationBBKey) VectorValue))

(fn UpdateLostTargetData
  (params (VectorValue :type Vector))
  (Utilities|FlowControl|Sequence
    (:then_0
      (CallFunction|UpdateTargetActor))
    (:then_1
      (CallFunction|UpdateLostTargetLocation VectorValue))))

(fn CheckIsSoundIsEnoughtoAlert?
  (params (SoundStrength :type Float%20%28single-precision%29))
  (return (>= SoundStrength (Variables|Default|GetMinSoundStrengthForAlert))))

(fn CheckSoundIsHearable?
  (params (SoundStrength :type Float%20%28single-precision%29))
  (return (> SoundStrength 0.0)))

(fn UpdateHeardShotLocation
  (params (VectorValue :type Vector))
  (AI|Components|Blackboard|SetValueasVector (Variables|Default|GetBlackboard) (Variables|Blackboard|GetHeardShotLocationBBKey) VectorValue))

(fn UpdateHeardShotStrengthType
  (params (EnumValue :type Byte))
  (AI|Components|Blackboard|SetValueasEnum (Variables|Default|GetBlackboard) (Variables|Blackboard|GetHeardShotStrengthBBKey) EnumValue))

(fn ComputeNewRoute
  (bind _returnvalue (Game|ConstructObjectfromClass "/Game/CompassoFPS/Core/Blueprints/Enemies/BP_Route.BP_Route_C" self))
  (CallFunction|AddRandomItemsfromSource (Variables|/Game/CompassoFPS/Core/Blueprints/Enemies/BP_Route.BP_Route_C|GetPoints _returnvalue) (Variables|Routing|GetUsableWaypoints) (CallFunction|ComputeRouteLength))
  (return _returnvalue))

(fn ComputeTargetBasedRoute
  (bind _tempallwaypoints (LocalVariables|GetTempAllWaypoints))
  (Utilities|Array|Clear _tempallwaypoints)
  (Utilities|Array|AppendArray _tempallwaypoints (Variables|Routing|GetAllWaypoints))
  (bind _returnvalue (Game|ConstructObjectfromClass "/Game/CompassoFPS/Core/Blueprints/Enemies/BP_Route.BP_Route_C" self))
  (for _index (range 1 (Variables|Routing|GetTargetSeekingRouteLength))
    (bind __ (CallFunction|GetNearestWaypoint (AI|Components|Blackboard|GetValueasVector (Variables|Default|GetBlackboard) (Variables|Blackboard|GetLostTargetLocationBBKey)) (LocalVariables|GetTempAllWaypoints)))
    (Utilities|Array|Add (Variables|/Game/CompassoFPS/Core/Blueprints/Enemies/BP_Route.BP_Route_C|GetPoints _returnvalue) __)
    (Utilities|Array|RemoveItem (LocalVariables|GetTempAllWaypoints) __))
  (return _returnvalue))