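; Behavior tree task that picks an enemy's next target location along the BP_Route stored in the blackboard.
; It increments the route point index, then re-reads it and looks up the point one past the stored value.
; A valid point's actor location becomes the target location and the task succeeds.
; When the points run out it clears the current route and fails, as it does without a route.
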(event EventReceiveExecuteAI
  (params (OwnerController :type AI%20Controller%20Object%20Reference) (ControlledPawn :type Pawn%20Object%20Reference))
  (bind _currentroutepointindexkey (Variables|Default|GetCurrentRoutePointIndexKey))
  (bind _returnvalue (Class|BTFunctionLibrary|GetBlackboardValueasInt _currentroutepointindexkey))
  (bind _returnvalue_2 (+ _returnvalue 1))
  (bind _asbp_route (Utilities|Casting|CastToBP_Route (Class|BTFunctionLibrary|GetBlackboardValueasObject (Variables|Default|GetCurrentRouteKey)))
    (:then
      (Class|BTFunctionLibrary|SetBlackboardValueasInt (Variables|Default|GetCurrentRoutePointIndexKey) _returnvalue_2)
      (if (Utilities|Array|IsValidIndex (Variables|/Game/CompassoFPS/Core/Blueprints/Enemies/BP_Route.BP_Route_C|GetPoints _asbp_route) _returnvalue_2)
        (AI|BehaviorTree|SetBlackboardValueasVector (Variables|Default|GetTargetLocationKey) (Transformation|GetActorLocation (Utilities|Array|Get(acopy) (Variables|/Game/CompassoFPS/Core/Blueprints/Enemies/BP_Route.BP_Route_C|GetPoints _asbp_route) _returnvalue_2)))
        (AI|BehaviorTree|FinishExecute true)
        (else
          (Class|BTFunctionLibrary|ClearBlackboardValue (Variables|Default|GetCurrentRouteKey))
          (AI|BehaviorTree|FinishExecute false))))
    (:CastFailed
      (AI|BehaviorTree|FinishExecute false))))