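; Simple AI enemy actor for the FPS, with health, a child-actor weapon, alert states and a start-point marker spawned on BeginPlay.
; TryBurst fires a random number of shots through a delay loop, blocking new bursts until the current one ends.
; SetAlertState shows the matching state icon and hides the rest, while helpers drive a reposition timer widget.
; Damage feeds the Health component, whose death event plays sounds and destroys the actor.
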(event OnDeath(Health)
  (bind _self self)
  ;[0 0.8828 1] Death
  (CallFunction|PlayGenericDeathSounds _self)
  (CallFunction|PrintDeath _self)
  (Actor|DestroyActor))

(event Custom|TryBurst
  ;[0.8984 0 1] Burst
  (if (Variables|Shooting|GetCanBurst?)
    (Variables|Shooting|SetCanBurst? false)
    (bind _output_get (Variables|Default|SetTempBurstShotCount (Shooting|ComputeBurstShotCount)))
    (if (> _output_get 0) :!label _label
      (Shooting|TryFire)
      (Math|Integer|DecrementInt (Variables|Default|GetTempBurstShotCount)
        (:%20%20
          (Utilities|FlowControl|Delay (Variables|Shooting|GetShotInterval))
          (goto _label)))
      (else
        (Variables|Shooting|SetCanBurst? true)))
    (else
      (Development|PrintString "Cant burst"))))

(event Game|Damage|EventAnyDamage
  (params (Damage :type Float%20%28single-precision%29) (DamageType :type Damage%20Type%20Object%20Reference) (InstigatedBy :type Controller%20Object%20Reference) (DamageCauser :type Actor%20Object%20Reference))
  ;[0.7812 1 0] Any Damage
  (Default|TakeDamage (Variables|Default|GetHealth) Damage))

(event EventBeginPlay
  ;[0 0.8594 1] Begin
  (CallFunction|CacheWeapon)
  (CallFunction|CacheStartValues))

(fn ConstructionScript)

(fn CacheWeapon
  (bind _asbp_weapon (Utilities|Casting|CastToBP_Weapon (Variables|/Script/Engine.ChildActorComponent|GetChildActor (Variables|Default|GetWeaponChild))))
  (bind _output_get (Variables|Shooting|SetWeapon _asbp_weapon))
  (Variables|/Game/CompassoFPS/Core/Blueprints/Weapons/BP_Weapon.BP_Weapon_C|SetShotPoint _output_get (Variables|Default|GetShotPoint)))

(fn ComputeBurstShotCount
  (return (Math|Random|RandomIntegerinRange (Variables|Shooting|GetMinBurstShotCount) (Variables|Shooting|GetMaxBurstShotCount))))

(fn ShowEyeIcon
  (Icons|ShowStateIcon (Variables|Default|GetEyeIcon)))

(fn ShowAlertIcon
  (Icons|ShowStateIcon (Variables|Default|GetAlertIcon)))

(fn ShowInvisibleIcon
  (Icons|ShowStateIcon (Variables|Default|GetInvisibleIcon)))

(fn ShowStateIcon
  (params (ToEnable :type Billboard%20Component%20Object%20Reference))
  (for _array_element (Components|GetChildrenComponents (Variables|Default|GetIcons) true)
    (if (== _array_element ToEnable)
      (Rendering|SetVisibility _array_element true true)
      (else
        (Rendering|SetVisibility _array_element false true)))))

(fn HideAllIcons
  (for _array_element (Components|GetChildrenComponents (Variables|Default|GetIcons) false)
    (Rendering|SetVisibility _array_element false true)))

(fn CacheStartValues
  (bind _returnvalue (Transformation|GetActorTransform))
  (bind _returnvalue_2 (Game|SpawnActorfromClass "/Script/Engine.TargetPoint" (Math|Transform|MakeTransform (.location _returnvalue) (.rotation _returnvalue) "1,1,1") "Undefined" 0 0))
  (Variables|Default|SetStartPoint _returnvalue_2))

(fn UpdateRepositionTimerText
  (params (Value :type Float%20%28single-precision%29))
  (Rendering|Components|TextRender|SetText (Variables|Default|GetTextRender) (Utilities|Text|ToText(Float) Value "HalfToEven" false true 1 324 0 1)))

(fn HideRepositionWidget
  (Rendering|SetVisibility (Variables|Default|GetRepositionWidget) false true))

(fn ShowRepositionWidget
  (Rendering|SetVisibility (Variables|Default|GetRepositionWidget) true true))

(fn TryFire
  (Default|TryFire (Variables|Shooting|GetWeapon)))

(fn SetAlertState
  (params (%20 :type BPE_AlertState%20Enum :default "NewEnumerator0"))
  (bind _output_get (Variables|Default|SetAlertState %20))
  (CallFunction|SetAlertStateIcon _output_get))

(fn ShowShootingIcon
  (Icons|ShowStateIcon (Variables|Default|GetShootingIcon)))

(fn SetAlertStateIcon
  (params (State :type BPE_AlertState%20Enum :default "NewEnumerator0"))
  (switch Utilities|FlowControl|Switch|SwitchonBPE_AlertState State
    (:NewEnumerator0
      (Icons|ShowInvisibleIcon))
    (:NewEnumerator1
      (Icons|ShowEyeIcon))
    (:NewEnumerator2
      (Icons|ShowShootingIcon))
    (:NewEnumerator3
      (Icons|ShowAlertIcon))))