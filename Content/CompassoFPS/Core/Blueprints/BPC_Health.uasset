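; Health actor component that tracks an owner's hit points and death state.
; On BeginPlay, Current is filled to Max.
; TakeDamage subtracts damage while alive, clamping at zero, then sets IsDead and fires the OnDeath dispatcher once so other logic can react.
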(event EventBeginPlay
  ;[1 1 1] Begin
  (Variables|Default|SetCurrent (Variables|Default|GetMax)))

(fn TakeDamage
  (params (Value :type Float%20%28single-precision%29))
  (if (not (Variables|Default|GetIsDead?))
    (if (> (- (Variables|Default|GetCurrent) Value) 0.0)
      (Variables|Default|SetCurrent (- (Variables|Default|GetCurrent) Value))
      (else
        (Variables|Default|SetCurrent 0.0)
        (Variables|Default|SetIsDead? true)
        (Default|CallOnDeath)))))