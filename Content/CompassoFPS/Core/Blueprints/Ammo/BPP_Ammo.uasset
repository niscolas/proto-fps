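; BPP_Ammo is an interactable ammo pickup that gives extra ammo to the player's current weapon.
; Interaction events toggle the PickIndicator's visibility as an interactor is added or removed.
; On interaction, it resolves the BP_FirstPersonCharacter owning the interactor component and calls AddExtraAmmo with AmountValue if the current weapon's type matches TargetType.
; The pickup destroys itself only when the ammo is successfully added.
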(event EventOnInteractorAdded
  (params (PossibleInteractor :type BPI%20Interactor%20Interface))
  ;[1 1 1] On Possible Interaction Begin
  (Rendering|SetVisibility (Variables|Default|GetPickIndicator) true true))

(event EventOnInteractorRemoved
  (params (PossibleInteractor :type BPI%20Interactor%20Interface))
  ;[1 1 1] On Possible Interaction End
  (Rendering|SetVisibility (Variables|Default|GetPickIndicator) false true))

(event EventOnInteraction
  (params (Interactor :type BPI%20Interactor%20Interface))
  ;[1 1 1] Interaction
  (CallFunction|InteractionCallback Interactor))

(fn ConstructionScript)

(fn TryAddExtraAmmo
  (params (Interactor :type BPI%20Interactor%20Interface))
  (bind _asbpc_interactor (Utilities|Casting|CastToBPC_Interactor Interactor))
  (bind _asbp_first_person_character (Utilities|Casting|CastToBP_FirstPersonCharacter (Components|GetOwner _asbpc_interactor)))
  (Utilities|IsValid (Variables|/Game/CompassoFPS/Core/Blueprints/BP_FirstPersonCharacter.BP_FirstPersonCharacter_C|GetCurrentWeapon _asbp_first_person_character)
    (:Is%20Valid
      (if (Utilities|Enum|Equal(Enum) (Variables|/Game/CompassoFPS/Core/Blueprints/Weapons/BP_Weapon.BP_Weapon_C|GetType (Variables|/Game/CompassoFPS/Core/Blueprints/BP_FirstPersonCharacter.BP_FirstPersonCharacter_C|GetCurrentWeapon _asbp_first_person_character)) (Variables|Default|GetTargetType))
        (bind _added (Default|AddExtraAmmo _asbp_first_person_character (Variables|Default|GetAmountValue)))
        (return _added)))))

(fn InteractionCallback
  (params (Interactor :type BPI%20Interactor%20Interface))
  (bind _added (CallFunction|TryAddExtraAmmo Interactor))
  (if _added
    (Actor|DestroyActor)))