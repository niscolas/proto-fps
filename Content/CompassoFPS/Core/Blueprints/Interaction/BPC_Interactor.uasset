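; BPC_Interactor is an interaction component that tracks a current interactable and lets it be triggered.
; Possible-interactable added and removed events cast to BPI_Interactable, fire the matching dispatcher and notify that object of the interactor.
; Both events store the object as CurrentInteractable, so removal leaves it set rather than clearing it.
; TryInteract calls OnInteraction on the stored interactable if it is still valid, passing itself.
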(event EventOnPossibleInteractableAdded
  (params (PossibleInteractable :type Object%20Object%20Reference))
  ;[1 1 1] Interactable Added
  (bind _asbpi_interactable (Utilities|Casting|CastToBPI_Interactable PossibleInteractable))
  (bind _output_get (Variables|Default|SetCurrentInteractable _asbpi_interactable))
  (Default|CallOnInteractableAdded _output_get)
  (Default|OnInteractorAdded _output_get self))

(event EventOnPossibleInteractableRemoved
  (params (PossibleInteractable :type Object%20Object%20Reference))
  ;[1 1 1] Interactable Removed
  (bind _asbpi_interactable (Utilities|Casting|CastToBPI_Interactable PossibleInteractable))
  (bind _output_get (Variables|Default|SetCurrentInteractable _asbpi_interactable))
  (Default|CallOnInteractableRemoved _output_get)
  (Default|OnInteractorRemoved _output_get self))

(fn TryInteract
  (bind _currentinteractable (Variables|Default|GetCurrentInteractable))
  (Utilities|IsValid (Utilities|ToObject(Interface) _currentinteractable)
    (:Is%20Valid
      (Default|OnInteraction _currentinteractable self))))