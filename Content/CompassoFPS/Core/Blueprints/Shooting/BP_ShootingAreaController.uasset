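; Shooting area controller that spawns enemy targets and lets the player reset them through interaction.
; On BeginPlay it spawns an enemy at every spawn point actor of the configured class in the level and tracks them in an array.
; Interacting destroys any surviving targets, clears the array and respawns the full set.
; A pick indicator shows while an interactor is present.
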(event EventOnInteractorRemoved
  (params (PossibleInteractor :type BPI%20Interactor%20Interface))
  ;[0.2656 1 0] On Interaction End
  (Rendering|SetVisibility (Variables|Default|GetPickIndicator) false true))

(event EventOnInteractorAdded
  (params (PossibleInteractor :type BPI%20Interactor%20Interface))
  ;[1 0 0.75] On Interaction Begin
  (Rendering|SetVisibility (Variables|Default|GetPickIndicator) true true))

(event EventBeginPlay
  ;[0 0.3906 1] Begin
  (CallFunction|SpawnTargets))

(event EventOnInteraction
  (params (Interactor :type BPI%20Interactor%20Interface))
  ;[1 0 0.7031] On Interaction
  (CallFunction|ReloadTargets))

(fn ConstructionScript)

(fn SpawnTargets
  (bind _outactors (Actor|GetAllActorsOfClass (Variables|Default|GetEnemiesSpawnPointClass)))
  (for _array_element _outactors
    (bind _returnvalue (Game|SpawnActorfromClass (Variables|Default|GetEnemiesClass) (Transformation|GetActorTransform _array_element) "Undefined" 0 0))
    (Utilities|Array|Add (Variables|Default|GetExistingTargets) _returnvalue)))

(fn DestroyTargets
  (bind _existingtargets (Variables|Default|GetExistingTargets))
  (for _array_element _existingtargets
    (Utilities|IsValid _array_element
      (:Is%20Valid
        (Actor|DestroyActor _array_element))))
  (Utilities|Array|Clear _existingtargets))

(fn ReloadTargets
  (CallFunction|DestroyTargets)
  (CallFunction|SpawnTargets))