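; Shotgun weapon Blueprint for CompassoFPS that replaces the inherited firing behavior with a multi-pellet hitscan shot.
; Each shot sets the offset randomization to its maximum, then fires a random number of raycasts between the minimum and maximum shot counts.
; Each successful raycast attempts to damage the hit actor, and the single-shot notification runs once after the whole volley.
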(event EventFire
  (CallFunction|FireOverride))

(fn ConstructionScript
  (|CallParentFunction))

(fn FireOverride
  (CallFunction|SetShotOffsetRandomization)
  (for _index (range 0 (CallFunction|ComputeShotCount))
    (bind (_outhit _returnvalue) (CallFunction|FireRaycast))
    (if _returnvalue
      (CallFunction|TryDamageHitActor _outhit)))
  (Default|CallOnSingleShot))

(fn ComputeShotCount
  (return (Math|Random|RandomIntegerinRange (Variables|Default|GetMinShotCount) (Variables|Default|GetMaxShotCount))))

(fn SetShotOffsetRandomization
  (Variables|Default|SetCurrentShotOffsetRandomization (Variables|Default|GetMaxShotOffsetRandomization)))