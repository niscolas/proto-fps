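; BP_PickableWeapon is a world weapon pickup that gives a first-person character a weapon when interacted with.
; It applies its configured skeletal mesh at BeginPlay and shows or hides a pick indicator as interactors are added or removed.
; On interaction, it spawns the weapon class with the character as owner and its camera as shot point, calls PickWeapon, then destroys itself.
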(event EventBeginPlay
  ;[1 0.7266 0] Begin Play
  (Class|SkinnedMeshComponent|SetSkeletalMesh (Variables|Default|GetSkeletalMesh) (Variables|Default|GetWeaponMesh) true))

(event EventOnInteractorRemoved
  (params (PossibleInteractor :type BPI%20Interactor%20Interface))
  ;[0 1 0.6719] Interaction
  (Rendering|SetVisibility (Variables|Default|GetPickIndicator) false true))

(event EventOnInteractorAdded
  (params (PossibleInteractor :type BPI%20Interactor%20Interface))
  ;[0 1 0.6719] Interaction
  (Rendering|SetVisibility (Variables|Default|GetPickIndicator) true true))

(event EventOnInteraction
  (params (Interactor :type BPI%20Interactor%20Interface))
  ;[0 1 0.6719] Interaction
  (bind _asbpc_interactor (Utilities|Casting|CastToBPC_Interactor Interactor))
  (bind _asbp_first_person_character (Utilities|Casting|CastToBP_FirstPersonCharacter (Components|GetOwner _asbpc_interactor))
    (:then
      (bind _returnvalue (Game|SpawnActorfromClass (Variables|Default|GetWeapon) (Transformation|GetActorTransform _asbp_first_person_character) "Undefined" _asbp_first_person_character (Variables|/Game/CompassoFPS/Core/Blueprints/BP_FirstPersonCharacter.BP_FirstPersonCharacter_C|GetCamera _asbp_first_person_character) 0))
      (Default|PickWeapon _asbp_first_person_character _returnvalue)
      (Actor|DestroyActor))
    (:CastFailed
      (Development|PrintString "Isn't FPS CHAR"))))

(fn ConstructionScript)