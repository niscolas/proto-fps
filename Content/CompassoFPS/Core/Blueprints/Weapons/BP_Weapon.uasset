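; Hitscan weapon actor that handles automatic fire, magazine and reserve ammo, and reloading.
; StartShooting runs a Delay loop that fires while held, widening random spread each repeat until StopShooting resets it.
; Each shot line-traces from ShotPoint, applying damage and a decal on hit, then plays sound and optionally reports noise to AI perception.
; Dispatchers signal shots and empty magazines, while failed reload checks only print messages.
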(event Custom|StartShooting
  ;[0.5 0 1] Shooting
  (Variables|Default|SetIsShooting? true)
  (Shooting|TryFire)
  (Utilities|FlowControl|Delay (Variables|Default|GetShotDelay) :!label _label)
  (if (Variables|Default|GetIsShooting?)
    (Shooting|IncreaseShotOffsetRandomization)
    (Shooting|TryFire)
    (goto _label)))

(event Custom|StopShooting
  ;[0.5 0 1] Shooting
  (Variables|Default|SetIsShooting? false)
  (Shooting|ResetShotOffsetRandomization))

(event EventBeginPlay
  ;[0.5938 0 1] Begin
  (AmmoRelated|FillAllAmmo))

(fn ConstructionScript)

(fn ResetShotOffsetRandomization
  (Variables|Default|SetCurrentShotOffsetRandomization "0, 0, 0"))

(fn TryFire
  (if (Shooting|CheckHasAmmo?)
    (AmmoRelated|DecreaseAmmo)
    (Shooting|Fire)
    (Shooting|PlayShotFX)
    (else
      (Default|CallOnNoAmmo))))

(fn ComputeShotOffset
  (bind _currentshotoffsetrandomization (Variables|Default|GetCurrentShotOffsetRandomization))
  (bind _baseshotoffset (Variables|Default|GetBaseShotOffset))
  (bind (_x _y _z) (Math|Vector|BreakVector _currentshotoffsetrandomization))
  (bind (_x_2 _y_2 _z_2) (Math|Vector|BreakVector _baseshotoffset))
  (return (Math|Vector|MakeVector (CallFunction|Randomize _x_2 _x) (CallFunction|Randomize _y_2 _y) (CallFunction|Randomize _z_2 _z))))

(fn PlayShotFX
  (Audio|PlaySoundatLocation (Variables|Default|GetShotSound) (Transformation|GetActorLocation) "0, 0, 0" 1.0 1.0 0.0 0 0 0)
  (if (Variables|Default|GetShouldReportNoise?)
    (Shooting|ReportNoise)))

(fn ComputeShotEndPoint
  (bind _shotpoint (Variables|Default|GetShotPoint))
  (bind _returnvalue (Transformation|GetWorldTransform _shotpoint))
  (return (+ (Shooting|ComputeShotOffset) (.location _returnvalue) (* (Math|Vector|GetForwardVector (.rotation _returnvalue)) (Variables|Default|GetShootDistance)))))

(fn CheckHasAmmo?
  (return (> (Variables|Default|GetCurrentMagazineAmmo) 0)))

(fn CheckCanReload?
  (bind _returnvalue (AmmoRelated|CheckNeedReload?))
  (bind _returnvalue_2 (AmmoRelated|CheckHasExtraAmmo?))
  (return (and _returnvalue_2 _returnvalue)))

(fn OnReloadStarted)

(fn CheckNeedReload?
  (bind _currentmagazineammo (Variables|Default|GetCurrentMagazineAmmo))
  (bind _maxmagazineammo (Variables|Default|GetMaxMagazineAmmo))
  (bind _returnvalue (< _currentmagazineammo _maxmagazineammo))
  (if _returnvalue
    _
    (else
      (AmmoRelated|OnAmmoFull)))
  (return _returnvalue))

(fn CheckHasExtraAmmo?
  (bind _currentextraammo (Variables|Default|GetCurrentExtraAmmo))
  (bind _returnvalue (> _currentextraammo 0))
  (if _returnvalue
    _
    (else
      (AmmoRelated|OnNoExtraAmmo)))
  (return _returnvalue))

(fn OnAmmoFull
  (Development|PrintString "Ammo already full ;-;"))

(fn OnNoExtraAmmo
  (Development|PrintString "There's no extra ammo "))

(fn Reload
  (bind _returnvalue (AmmoRelated|ComputeMagazineAmmoNeeded))
  (if (<= _returnvalue (Math|Integer|Clamp(Integer) (Variables|Default|GetCurrentExtraAmmo) 0 (Variables|Default|GetMaxMagazineAmmo)))
    (AmmoRelated|OnEnoughExtraAmmotoFullReload _returnvalue)
    (else
      (AmmoRelated|OnNotEnoughExtraAmmotoFullReload))))

(fn OnEnoughExtraAmmotoFullReload
  (params (AmmoNeeded :type Integer))
  (Variables|Default|SetCurrentMagazineAmmo (+ AmmoNeeded (Variables|Default|GetCurrentMagazineAmmo)))
  (Variables|Default|SetCurrentExtraAmmo (- (Variables|Default|GetCurrentExtraAmmo) AmmoNeeded)))

(fn OnNotEnoughExtraAmmotoFullReload
  (Variables|Default|SetCurrentMagazineAmmo (+ (Variables|Default|GetCurrentMagazineAmmo) (Variables|Default|GetCurrentExtraAmmo)))
  (Variables|Default|SetCurrentExtraAmmo 0))

(fn FillAllAmmo
  (Variables|Default|SetCurrentExtraAmmo (Variables|Default|GetMaxExtraAmmo))
  (Variables|Default|SetCurrentMagazineAmmo (Variables|Default|GetMaxMagazineAmmo)))

(fn ComputeMagazineAmmoNeeded
  (return (- (Variables|Default|GetMaxMagazineAmmo) (Variables|Default|GetCurrentMagazineAmmo))))

(fn AddExtraAmmo
  (params (AmmoCount :type Integer))
  (bind _maxextraammo (Variables|Default|GetMaxExtraAmmo))
  (if (== (Variables|Default|GetCurrentExtraAmmo) _maxextraammo)
    (return false)
    (else
      (Variables|Default|SetCurrentExtraAmmo (Math|Integer|Clamp(Integer) (+ AmmoCount (Variables|Default|GetCurrentExtraAmmo)) 0 _maxextraammo))
      (return true))))

(fn Fire
  (bind (_outhit _returnvalue) (Shooting|FireRaycast))
  (Default|CallOnSingleShot)
  (if _returnvalue
    (Shooting|TryDamageHitActor _outhit)))

(fn IncreaseShotOffsetRandomization
  (Variables|Default|SetCurrentShotOffsetRandomization (+ (Variables|Default|GetPerShotOffsetRandomization) (Variables|Default|GetCurrentShotOffsetRandomization))))

(fn DecreaseAmmo
  (if (not (Variables|Default|GetHasUnlimitedAmmo?))
    (Math|Integer|DecrementInt (Variables|Default|GetCurrentMagazineAmmo))))

(fn SpawnHitDecal
  (params (HitNormal :type Vector) (HitLocation :type Vector))
  (Rendering|Decal|SpawnDecalatLocation "/Game/CompassoFPS/Core/Materials/M_ShotDecal.M_ShotDecal" "10.000000,10.000000,10.000000" HitLocation (Math|Conversions|RotationFromXVector HitNormal) (Variables|Default|GetShotDecalLifetime)))

(fn FireRaycast
  (bind (_outhit _returnvalue) (Collision|LineTraceByChannel (.location (Transformation|GetWorldTransform (Variables|Default|GetShotPoint))) (Shooting|ComputeShotEndPoint) "TraceTypeQuery1" false 0 (Variables|Default|GetShotTraceDebugType) true "(R=1.000000,G=0.000000,B=0.000000,A=1.000000)" "(R=0.000000,G=1.000000,B=0.000000,A=1.000000)" 2.0))
  (return _outhit _returnvalue))

(fn TryDamageHitActor
  (params (Hit :type Hit%20Result%20Structure%20%28by%20ref%29))
  (bind (_bblockinghit _binitialoverlap _time _distance _location _impactpoint _normal _impactnormal _physmat _hitactor) (Collision|BreakHitResult Hit))
  (Shooting|SpawnHitDecal _impactnormal _impactpoint)
  (Game|Damage|ApplyDamage _hitactor (Variables|Default|GetShotDamage) 0 0))

(fn ReportNoise
  (Class|AISenseHearing|ReportNoiseEvent (Transformation|GetActorLocation) (Variables|Default|GetShotSoundLoudness) (Components|GetOwner) (Variables|Default|GetShotSoundMaxRange) "None"))