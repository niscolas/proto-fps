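; Grenade launcher weapon Blueprint that fires physics-driven explosive grenades.
; Its Fire event spawns the configured grenade class at ShootPoint's location and rotation at triple scale, passing in the explosion radius and impulse.
; It then launches the grenade by adding linear velocity to its sphere along ShotPoint's forward vector, scaled by ShotImpulse.
; The construction script only calls the parent's.
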(event EventFire
  (bind _shootpoint (Variables|Default|GetShootPoint))
  (bind _returnvalue (Transformation|GetWorldTransform _shootpoint))
  (bind _returnvalue_2 (Game|SpawnActorfromClass (Variables|Default|GetActualGrenade) (Math|Transform|MakeTransform (.location _returnvalue) (.rotation _returnvalue) "3.000000,3.000000,3.000000") "Undefined" 0 (Variables|Default|GetExplosionRadius) (Variables|Default|GetExplosionImpulse) 0))
  (Physics|SetPhysicsLinearVelocity (Variables|/Game/CompassoFPS/Core/Blueprints/Weapons/BP_Grenade.BP_Grenade_C|GetSphere _returnvalue_2) (* (Math|Vector|GetForwardVector (Variables|Default|GetShotPoint)) (Variables|Default|GetShotImpulse)) true "None"))

(fn ConstructionScript
  (|CallParentFunction))