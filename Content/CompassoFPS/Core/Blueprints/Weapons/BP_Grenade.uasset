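; BP_Grenade is a timed grenade actor that explodes after a configurable delay from BeginPlay.
; On detonation it spawns a BP_GrenadeExplosion at its transform, passing radius and impulse, and plays the explosion sound.
; It then applies flat damage to every actor found by a sphere overlap of the same radius, with no falloff or line-of-sight check, and destroys itself.
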(event EventBeginPlay
  (bind _returnvalue (Transformation|GetActorTransform))
  ;[0.5234 0 1] Begin
  (Utilities|FlowControl|Delay (Variables|Default|GetExplosionDelay))
  (Game|SpawnActorfromClass "/Game/CompassoFPS/Core/Blueprints/Weapons/BP_GrenadeExplosion.BP_GrenadeExplosion_C" (Math|Transform|MakeTransform (.location _returnvalue) (.rotation _returnvalue) "1,1,1") "Undefined" 0 (Variables|Default|GetExplosionRadius) (Variables|Default|GetExplosionImpulse) 0)
  (Audio|PlaySoundatLocation "/Game/CompassoFPS/Core/Weapons/Grenade/S_GrenadeExplosion.S_GrenadeExplosion" (Transformation|GetActorLocation) "0, 0, 0" 1.0 1.0 0.0 0 0 0)
  (bind _outactors (Collision|SphereOverlapActors (Transformation|GetActorLocation) (Variables|Default|GetExplosionRadius) (Variables|Default|GetObject%20Types) 0))
  (for _array_element _outactors
    (Game|Damage|ApplyDamage _array_element (Variables|Default|GetExplosionDamage) 0 0))
  (Actor|DestroyActor))

(fn ConstructionScript)